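; BP_Functions is a demo Blueprint that explores functions and custom events through on-screen printing.
; On BeginPlay it prints an intro, calls the random-colored Say event and CountToNumber, then prints each entry in Names.
; GetColorByNameLength shades each name from black to white as its length grows.
; CountToNumber's loop body is empty, as its indexed Say call is disconnected.
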(event Custom|Say
  (params (In%20String :type String) (Duration :type Float%20%28double-precision%29))
  (Development|PrintString In%20String true true (Utilities|Struct|MakeLinearColor (Math|Random|RandomFloat) (Math|Random|RandomFloat) (Math|Random|RandomFloat) 1.0) Duration))

(event EventBeginPlay
  (Development|PrintString "We are exploring functions today!")
  (CallFunction|Say "" 0.0)
  (CallFunction|CounttoNumber)
  (for _array_element (Variables|Default|GetNames)
    (bind _output (CallFunction|GetColorbyNameLength _array_element))
    (Development|PrintString _array_element true true _output)))

(fn ConstructionScript)

(fn CounttoNumber
  (params (Number :type Integer))
  (for _index (range 0 Number)
    _)
  (return))

(fn GetColorbyNameLength
  (params (Input :type String))
  (bind _returnvalue (Utilities|String|Len Input))
  (bind _returnvalue_2 (- _returnvalue 5.0))
  (bind _returnvalue_3 (* _returnvalue_2 0.2))
  (if (<= _returnvalue 5)
    (LocalVariables|SetNewLocalVar (Utilities|Struct|MakeLinearColor 0.0 0.0 0.0 1.0))
    (elif (>= _returnvalue 10)
      (LocalVariables|SetNewLocalVar (Utilities|Struct|MakeLinearColor 1.0 1.0 1.0 1.0))
      (else
        (LocalVariables|SetNewLocalVar (Utilities|Struct|MakeLinearColor _returnvalue_3 _returnvalue_3 _returnvalue_3 1.0)))))
  (return (LocalVariables|GetNewLocalVar)))