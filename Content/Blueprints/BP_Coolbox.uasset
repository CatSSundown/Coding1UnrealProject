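; BP_Coolbox is a test-style actor that continuously spawns BP_Key actors above its Cube component.
; On BeginPlay it caches a position above the cube and prints debug messages with its name and that position.
; It then loops indefinitely through SpawnActor and Delay at that fixed point, with a random scale whose range is zero, so the spawn scale evaluates to zero.
; Overlap, Tick and construction logic are empty.
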(event EventBeginPlay
  (Variables|Default|SetKeySpawnPosition (+ (Transformation|GetWorldLocation (Variables|Default|GetCube)) "0.000000,0.000000,200.000000"))
  (Development|PrintString (Utilities|String|Append (Utilities|GetDisplayName self) " Exists") true true "(R=0.000000,G=0.660000,B=1.000000,A=1.000000)" 1e+01)
  (Development|PrintString (Utilities|String|ToString(Vector) (Variables|Default|GetKeySpawnPosition)) true true "(R=0.002954,G=1.000000,B=0.000000,A=1.000000)" 1e+01)
  (Development|PrintString (Utilities|String|ToString(Vector) (Variables|Default|GetKeySpawnPosition)) true true "(R=1.000000,G=0.000000,B=0.094928,A=1.000000)")
  (Game|SpawnActorfromClass "/Game/Blueprints/BP_Key.BP_Key_C" (Math|Transform|MakeTransform (Variables|Default|GetKeySpawnPosition) "0, 0, 0" (* (Math|Random|RandomFloatinRange 0.0 0.0) 1.0)) "Undefined" "MultiplyWithRoot" 0 0 :!label _label)
  (Utilities|FlowControl|Delay (Variables|Default|GetDuration))
  (goto _label))

(event Collision|EventActorBeginOverlap
  (params (OtherActor :type Actor%20Object%20Reference)))

(event EventTick
  (params (DeltaSeconds :type Float%20%28single-precision%29)))

(fn ConstructionScript)