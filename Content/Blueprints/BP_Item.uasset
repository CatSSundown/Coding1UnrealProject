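; BP_Item is an item Blueprint with a name, elemental type and damage, which prints debug messages on BeginPlay.
; Its Constructor function, called at BeginPlay, picks a random name from four literals, with an index range reaching one past the end.
; GetDamage uses a modulo-4 offset to detect opposing elements and doubles the Damage variable itself, but returns the value saved beforehand.
; An element match branch is left unconnected.
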(event EventBeginPlay
  (CallFunction|Constructor)
  (Development|PrintString (Utilities|String|Append "Hello! My name is " (Variables|Default|GetName)))
  (bind _damage (CallFunction|GetDamage "NewEnumerator3"))
  (Development|PrintString (Utilities|String|Append "our elem type is " (Utilities|String|EnumtoString (Variables|Default|GetElementalType)) " victim is air, damage = " (Utilities|String|ToString(Integer) _damage)) true true "(R=1.000000,G=0.015463,B=0.000000,A=1.000000)" 5.0))

(event Collision|EventActorBeginOverlap
  (params (OtherActor :type Actor%20Object%20Reference)))

(event EventTick
  (params (DeltaSeconds :type Float%20%28single-precision%29)))

(fn ConstructionScript)

(fn Constructor
  (bind _returnvalue (Utilities|String|MakeLiteralString "Josh"))
  (bind _returnvalue_2 (Utilities|String|MakeLiteralString "Berto"))
  (bind _returnvalue_3 (Utilities|String|MakeLiteralString "Dai"))
  (bind _returnvalue_4 (Utilities|String|MakeLiteralString "Hart"))
  (bind _array (Utilities|Array|MakeArray _returnvalue_2 _returnvalue_3 _returnvalue_4 _returnvalue))
  (if true
    (Utilities|Array|Shuffle _array)
    (Variables|Default|SetName (Utilities|Array|Get(acopy) _array (Math|Random|RandomIntegerinRange 0 (- (Utilities|Array|Length _array) 0))))))

(fn GetDamage
  (params (Victim%20Element%20Type :type ElementalType%20Enum :default "NewEnumerator1"))
  (LocalVariables|SetReturn%20Damage (Variables|Default|GetDamage))
  (if (== (Class|KismetMathLibrary|PercentByteByte (+ Victim%20Element%20Type 2) 4) (Variables|Default|GetElementalType))
    (Variables|Default|SetDamage (* (Variables|Default|GetDamage) 2)))
  (return (LocalVariables|GetReturn%20Damage)))