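; BP_Enemy is an enemy actor that dies when the third-person player character overlaps its capsule.
; The overlap sets Health negative, and a looping Delay started on BeginPlay polls Health several times a second to destroy the actor.
; BeginPlay also applies EnemyTeamMaterial to the body when set; otherwise it only shuffles Materials without applying one.
; The Names array is shuffled but never used.
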(event OnComponentBeginOverlap(Capsule)
  (params (OverlappedComponent :type Primitive%20Component%20Object%20Reference) (OtherActor :type Actor%20Object%20Reference) (OtherComp :type Primitive%20Component%20Object%20Reference) (OtherBodyIndex :type Integer) (bFromSweep :type Boolean) (SweepResult :type Hit%20Result%20Structure%20%28by%20ref%29))
  (Utilities|Casting|CastToBP_ThirdPersonCharacter OtherActor) ; Did the player hit the enemy?
  (Variables|Default|SetHealth -1.0))

(event EventBeginPlay
  (Utilities|FlowControl|Sequence
    (:then_0
      ;[1 0.3265 0.3524] Every .2 seconds, check if hp is <= 0. If true, destroy self
      (Utilities|FlowControl|Delay 0.2 :!label _label)
      (if (<= (Variables|Default|GetHealth) 0.0)
        (Actor|DestroyActor)
        (else
          (goto _label))))
    (:then_1
      (Utilities|Array|Shuffle (Variables|Default|GetNames)))
    (:then_2
      (Utilities|IsValid (Variables|Default|GetEnemy%20Team%20Material)
        (:Is%20Valid
          (Development|PrintString "A Material has been set")
          (Rendering|Material|SetMaterial (Variables|Default|GetBody) 0 (Variables|Default|GetEnemy%20Team%20Material)) ; Set Selected Material
        )
        (:Is%20Not%20Valid
          (Development|PrintString "Let's pick a random material")
          (Utilities|Array|Shuffle (Variables|Default|GetMaterials)))))))

(event Collision|EventActorBeginOverlap
  (params (OtherActor :type Actor%20Object%20Reference)))

(event EventTick
  (params (DeltaSeconds :type Float%20%28single-precision%29)))

(fn ConstructionScript)